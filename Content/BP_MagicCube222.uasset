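; BP_MagicCube222 is the input layer for a 2x2x2 magic cube puzzle.
; Six input actions (F, B, L, R, U, D) each call RotateLayer with an axis, one of two layer indices and a signed quarter turn.
; Random runs a short Scramble and Reset calls ResetCube; the graph only forwards input, and the cube logic is defined outside it.
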(event `InputAction|RotateF`
  (params (Key :type "Key Structure"))
  (:`Pressed`
    (`self.RotateLayer` "X" 0 -90.0)))

(event `InputAction|Random`
  (params (Key :type "Key Structure"))
  (:`Pressed`
    (`self.Scramble` 3)))

(event `InputAction|Reset`
  (params (Key :type "Key Structure"))
  (:`Pressed`
    (`self.ResetCube`)))

(event `InputAction|RotateB`
  (params (Key :type "Key Structure"))
  (:`Pressed`
    (`self.RotateLayer` "X" 1 90.0)))

(event `InputAction|RotateL`
  (params (Key :type "Key Structure"))
  (:`Pressed`
    (`self.RotateLayer` "Y" 0 -90.0)))

(event `InputAction|RotateR`
  (params (Key :type "Key Structure"))
  (:`Pressed`
    (`self.RotateLayer` "Y" 1 90.0)))

(event `InputAction|RotateU`
  (params (Key :type "Key Structure"))
  (:`Pressed`
    (`self.RotateLayer` "Z" 1 90.0)))

(event `InputAction|RotateD`
  (params (Key :type "Key Structure"))
  (:`Pressed`
    (`self.RotateLayer` "Z" 0 -90.0)))

(fn `UserConstructionScript`)